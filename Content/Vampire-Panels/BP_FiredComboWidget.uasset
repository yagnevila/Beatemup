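; BP_FiredComboWidget is a Blueprint that hosts a WB_FiredCombo widget for displaying a combo in the game.
; On BeginPlay it casts its Widget component's widget to WB_FiredCombo and passes in the point count, points multiplier and TimeToSummDrop as the timer.
; A delayed path into the same setup exists but is never run, and the construction script is empty.
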(event `self.ReceiveBeginPlay`
  (bind _aswb_fired_combo (cast `/Game/Vampire-Panels/WB_FiredCombo` (`WidgetComponent.GetWidget` (`self.Widget`))))
  (set `/Game/Vampire-Panels/WB_FiredCombo.NumPoints` (`self.Num Points`) _aswb_fired_combo)
  (set `/Game/Vampire-Panels/WB_FiredCombo.PointsMultilpicator` (`self.Points Multilpicator`) _aswb_fired_combo)
  (set `/Game/Vampire-Panels/WB_FiredCombo.Timer` (`self.TimeToSumm&Drop`) _aswb_fired_combo))

(fn `UserConstructionScript`)