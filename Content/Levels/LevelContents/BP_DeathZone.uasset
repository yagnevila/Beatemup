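; BP_DeathZone is a furnace trigger that destroys stunned BP_StPanel_3 enemies and shows combo points for them.
; A qualifying overlap or hit on its Cube destroys the overlapping enemies, counting them over a one-second window.
; Points per enemy scale with group size, and a cumulative counter caps the popup loop.
; DoOnce-gated, the loop spawns stacked BP_FiredComboWidget actors on a socket that a Timeline moves upward between spawns.
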(event `self.Cube.OnComponentBeginOverlap`
  (params (OverlappedComponent :type "PrimitiveComponent Object Reference") (OtherActor :type "Actor Object Reference") (OtherComp :type "PrimitiveComponent Object Reference") (OtherBodyIndex :type Integer) (bFromSweep :type Boolean) (SweepResult :type "HitResult Structure (by ref)"))
  (bind _overlappingactors (`PrimitiveComponent.GetOverlappingActors` (`self.Cube`) "/Game/Vampire-Panels/BP_StPanel_3.BP_StPanel_3_C"))
  (bind _asbp_st_panel_3 (cast `/Game/Vampire-Panels/BP_StPanel_3` OtherActor :!label _label))
  (if (`/Game/Vampire-Panels/BP_StPanel_3.IsInStan` _asbp_st_panel_3)
    ;[1 1 1] Подсчёт врагов в группе и их уничножение.
    (set `self.HowMuchEnemy` (+ (`self.HowMuchEnemy`) (`KismetArrayLibrary.Array_Length` _overlappingactors)))
    (`self.K2_DestroyActor` _overlappingactors)
    ;[1 1 1] Периуд подсчёта группы. Объеденение Execution пути.
    (`KismetSystemLibrary.Delay` 1.0)
    ;[1 1 1] Подсчёт очков одного врага.
    (set `self.PointsOfOneEnemy` (* (`self.HowMuchEnemy`) 100))
    ;[1 1 1] Перевод счётчика врагов их абсолютный подсчёт для этой печи.
    (set `self.AbsoluteEnemyCounter` (+ (`self.HowMuchEnemy`) (`self.AbsoluteEnemyCounter`)))
    (set `self.HowMuchEnemy` 0)
    (`|ExecutionSequence`
      (:`then_0`
        (`KismetSystemLibrary.RetriggerableDelay` (* 0.25 (`self.AbsoluteEnemyCounter`)))
        (goto _label_2 :!via `Reset`))
      (:`then_1`
        (`/Engine/EditorBlueprintResources/StandardMacros.DoOnce` false :!label _label_2
          (:`Completed`
            (bind _counter (`/Engine/EditorBlueprintResources/StandardMacros.Do N` (`self.AbsoluteEnemyCounter`) :!label _label_3)
              (:`Exit`
                (bind _returnvalue (`|SpawnActorFromClass` "/Game/Vampire-Panels/BP_FiredComboWidget.BP_FiredComboWidget_C" (`KismetMathLibrary.MakeTransform` (0.0 0.0 0.0)) "Undefined" "MultiplyWithRoot" null 5.0 (`self.PointsOfOneEnemy`) 0 null))
                (`self.K2_AttachToComponent` _returnvalue (`self.Soket`) "None" "SnapToTarget" "KeepRelative" "KeepRelative" true)
                (`self.K2_AddActorLocalOffset` _returnvalue (`KismetMathLibrary.MakeVector` 0.0 0.0 (`KismetMathLibrary.Conv_IntToDouble` (* _counter -20))) false false)
                (`Timeline|Timeline` :!via `PlayFromStart`
                  (:`Update`
                    (`SceneComponent.K2_AddLocalOffset` (`self.Soket`) (`KismetMathLibrary.MakeVector` 0.0 0.0 (* (`GameplayStatics.GetWorldDeltaSeconds`) 60.0)) false false))
                  (:`Finished`
                    (`KismetSystemLibrary.Delay` 0.25)
                    (goto _label_3)))))))))))

(event `self.Cube.OnComponentHit`
  (params (HitComponent :type "PrimitiveComponent Object Reference") (OtherActor :type "Actor Object Reference") (OtherComp :type "PrimitiveComponent Object Reference") (NormalImpulse :type "Vector Structure") (Hit :type "HitResult Structure (by ref)"))
  (goto _label))

(fn `UserConstructionScript`)