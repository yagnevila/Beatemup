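; BP_WideKickBox+ is a short-lived hit box that knocks away BP_StPanel_3 actors inside its Box volume.
; One tick after BeginPlay it gathers the overlapping panels and calls PunchWithDelay on each, passing itself as the punching actor.
; The punch vector follows the Arrow component's world rotation, with strength scaled up from SpeedOfToss.
; The actor destroys itself after a delay of under a second.
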(event `self.ReceiveBeginPlay`
  (bind _overlappingactors (`PrimitiveComponent.GetOverlappingActors` (`self.Box`) "/Game/Vampire-Panels/BP_StPanel_3.BP_StPanel_3_C"))
  (`|ExecutionSequence`
    (:`then_0`
      (`KismetSystemLibrary.Delay` 0.9)
      (`self.K2_DestroyActor`))
    (:`then_1`
      (`KismetSystemLibrary.DelayUntilNextTick`)
      (set `self.Overlapping Enemys` _overlappingactors)
      (for _array_element _overlappingactors
        (bind _asbp_st_panel_3 (cast `/Game/Vampire-Panels/BP_StPanel_3` _array_element))
        (`/Game/Vampire-Panels/BP_StPanel_3.PunchWithDelay` _asbp_st_panel_3 (`KismetMathLibrary.GreaterGreater_VectorRotator` (`KismetMathLibrary.MakeVector` (* (`self.SpeedOfToss`) 5.0)) (`SceneComponent.K2_GetComponentRotation` (`self.Arrow`))) self)))))

(fn `UserConstructionScript`)