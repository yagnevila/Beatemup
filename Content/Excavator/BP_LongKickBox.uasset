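; BP_LongKickBox is a short-lived kick volume that stuns and shoves BP_StPanel_3 enemies along its arrow direction, destroying itself after a brief delay.
; One tick after spawning, it snapshots the box's overlapping actors and calls ToStan on those enemies.
; Tick repeatedly launches ungrouped ones at SpeedOfToss, adding sideways velocity proportional to their offset from the arrow's axis to pull them into line.
; Actors leaving the box drop from the list.
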(event `self.ReceiveBeginPlay`
  (bind _overlappingactors (`PrimitiveComponent.GetOverlappingActors` (`self.Box`) null))
  (`|ExecutionSequence`
    (:`then_0`
      (`KismetSystemLibrary.DelayUntilNextTick`)
      (set `self.Overlapping Enemys` _overlappingactors)
      (for _array_element _overlappingactors
        (bind _asbp_enemy (cast `/Game/Vampire-Panels/BP_StPanel_3` _array_element))
        (`/Game/Vampire-Panels/BP_StPanel_3.To Stan` _asbp_enemy (`KismetMathLibrary.GreaterGreater_VectorRotator` (`KismetMathLibrary.MakeVector` 1.0) (`SceneComponent.K2_GetComponentRotation` (`self.Arrow`))))))
    (:`then_1`
      (`KismetSystemLibrary.Delay` 1.4)
      (`self.K2_DestroyActor`))))

(event `self.ReceiveTick`
  (params (DeltaSeconds :type "Float (single-precision)"))
  (bind (_relativelocation_x _relativelocation_y) (`KismetMathLibrary.BreakVector` (`SceneComponent.RelativeLocation` (`self.Arrow`))))
  ;[1 1 1] Код отвечающий за толкание в определённом направлении.
  ;
  ; А также если толкаемы враг не на оси этого актора — то этот код толкает врага к центру. То есть стаблизирует линию врагов в линию.
  (if (not (`KismetArrayLibrary.Array_IsEmpty` (`self.Overlapping Enemys`)))
    (for _array_element (`self.Overlapping Enemys`)
      (if (`PrimitiveComponent.IsOverlappingActor` (`self.Box`) _array_element)
        (bind _asbp_enemy (cast `/Game/Vampire-Panels/BP_StPanel_3` _array_element :!pure true))
        (if (not (`/Game/Vampire-Panels/BP_StPanel_3.IsInGroup` _asbp_enemy))
          (bind (_returnvalue_x _returnvalue_y) (`KismetMathLibrary.BreakVector` (`KismetMathLibrary.InverseTransformLocation` (`self.GetTransform`) (`self.K2_GetActorLocation` _array_element))))
          (bind _returnvalue (- _returnvalue_y _relativelocation_y))
          (`Character.LaunchCharacter` _asbp_enemy (`KismetMathLibrary.GreaterGreater_VectorRotator` (`KismetMathLibrary.MakeVector` (`self.SpeedOfToss`) (`KismetMathLibrary.SelectFloat` 0.0 (* _returnvalue -1.0 15.0) (== _returnvalue 0.0))) (`SceneComponent.K2_GetComponentRotation` (`self.Arrow`))) false false))
        (else
          (`KismetArrayLibrary.Array_RemoveItem` (`self.Overlapping Enemys`) _array_element))))))

(event `self.Box.OnComponentEndOverlap`
  (params (OverlappedComponent :type "PrimitiveComponent Object Reference") (OtherActor :type "Actor Object Reference") (OtherComp :type "PrimitiveComponent Object Reference") (OtherBodyIndex :type Integer)))

(fn `UserConstructionScript`)