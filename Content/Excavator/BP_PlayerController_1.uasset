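; Player controller for the excavator game that handles saved progress, the pause menu and level progression.
; On BeginPlay it loads or creates the save, applies saved mouse sensitivity to the excavator, plays a fade widget and opens two media sources.
; The menu input toggles the main menu, cursor and pause outside MenuLevel.
; OpenNextLevel finds the current map in a levels data table, opens the following row and saves the highest unlocked index.
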(event `self.ReceiveBeginPlay`
  (`|ExecutionSequence`
    (:`then_0`
      (set `self.StartLevelLocation` (`self.GetTransform` (`GameplayStatics.GetPlayerPawn` 0)))
      (bind _returnvalue (`GameplayStatics.DoesSaveGameExist` (`self.StaticSaveName`)))
      (if _returnvalue
        (bind _returnvalue_2 (`GameplayStatics.LoadGameFromSlot` (`self.StaticSaveName`)))
        (bind _asbp_save_game (cast `/Game/Excavator/BP_SaveGame` _returnvalue_2))
        (bind _output_get (set `self.LastGameSave` _asbp_save_game))
        (`|ExecutionSequence`
          (:`then_0`
            (bind _asbp_excavator_2 (cast `/Game/Excavator/BP_Excavator_2` (`GameplayStatics.GetPlayerPawn` 0)))
            (set `/Game/Excavator/BP_Excavator_2.Mouse Sensetive Multiplayer` (`/Game/Excavator/BP_SaveGame.MouseSensitivity` _output_get) _asbp_excavator_2))
          (:`then_1`
            (set `self.Open Level Index` (`/Game/Excavator/BP_SaveGame.OpenLevelIndex` _output_get))))
        (else
          (bind _returnvalue_3 (`GameplayStatics.CreateSaveGameObject` "/Game/Excavator/BP_SaveGame.BP_SaveGame_C"))
          (set `self.LastGameSave` _returnvalue_3)
          (bind _indexlevel (`self.GetCurrentLevelIndex`))
          (set `/Game/Excavator/BP_SaveGame.OpenLevelIndex` _indexlevel (`self.LastGameSave`))
          (`self.SaveGame`))))
    (:`then_1`
      ;[1 1 1] То, как включается Fade Out, можно копировать в другие места. Для Fade Inпросто подставить другой виджет можно.
      (bind _returnvalue_4 (`|CreateWidget` "/Game/Interface/WB_FadeOut.WB_FadeOut_C" null 0.5))
      (`UserWidget.AddToViewport` _returnvalue_4 0)
      (`KismetSystemLibrary.Delay` 0.5))
    (:`then_2`
      (`|ExecutionSequence`
        (:`then_0`
          (`MediaPlayer.OpenSource` (`self.MediaPlayer_1`) "/Game/Interface/BoardersAndTextures/TextOpen.TextOpen"))
        (:`then_1`
          (`MediaPlayer.OpenSource` (`self.MediaPlayer_2`) "/Game/Interface/BoardersAndTextures/MS_LoopText.MS_LoopText"))))))

(event `InputAction|MenuOpenClose` :paused true
  (params (Key :type "Key Structure"))
  ;[1 1 1] Открытие и закрытие меню
  (:`Pressed`
    (bind _returnvalue (`GameplayStatics.GetCurrentLevelName` true :!label _label))
    (if (not (== _returnvalue "MenuLevel"))
      (`/Engine/EditorBlueprintResources/StandardMacros.IsValid` (`self.MainMenuReference`)
        (:`Is Valid`
          (`Widget.RemoveFromParent` (`self.MainMenuReference`))
          (set `self.MainMenuReference` null)
          (set `self.bShowMouseCursor` false)
          (`GameplayStatics.SetGamePaused` false))
        (:`Is Not Valid`
          (bind _returnvalue_2 (`|CreateWidget` "/Game/Interface/WB_MainMenu_4.WB_MainMenu_4_C" self))
          (set `self.MainMenuReference` _returnvalue_2)
          (`UserWidget.AddToViewport` _returnvalue_2 0)
          (set `self.bShowMouseCursor` true)
          (`GameplayStatics.SetGamePaused` true))))))

(event `UnPaused`
  ;[1 1 1] Открытие и закрытие меню
  (goto _label))

(fn `GetCurrentLevelIndex`
  (returns (IndexLevel :type Integer))
  (bind _returnvalue (`GameplayStatics.GetCurrentLevelName` true))
  (bind _outrownames (`DataTableFunctionLibrary.GetDataTableRowNames` "/Game/Levels/DT_Levels_Pre1.DT_Levels_Pre1"))
  (for (_array_element _array_index) _outrownames
    (bind _returnvalue_2 (`|GetDataTableRow` "/Game/Levels/DT_Levels_Pre1.DT_Levels_Pre1" _array_element)
      (:`then`
        (if (== _returnvalue (`.MapFileName_7_38EDD7FD448484FB78EF68B62B13310E` (break `/Game/Levels/Strct_Levels` _returnvalue_2)))
          (`|ExecutionSequence`
            (:`then_0`
              (return _array_index))
            (:`then_1`
              (break)))))))
  (return _array_index))

(fn `OpenNextLevel`
  (`|ExecutionSequence`
    (:`then_0`
      (`self.SaveGame`))
    (:`then_1`
      (bind _indexlevel (`self.GetCurrentLevelIndex`))
      (bind _outrownames (`DataTableFunctionLibrary.GetDataTableRowNames` "/Game/Levels/DT_Levels_Pre1.DT_Levels_Pre1"))
      (bind _returnvalue (+ _indexlevel 1))
      (bind _output (`|GetArrayItem` _outrownames _returnvalue))
      (if (!= _output "None")
        (bind _returnvalue_2 (`|GetDataTableRow` "/Game/Levels/DT_Levels_Pre1.DT_Levels_Pre1" _output)
          (:`then`
            (`GameplayStatics.OpenLevel` (`.MapFileName_7_38EDD7FD448484FB78EF68B62B13310E` (break `/Game/Levels/Strct_Levels` _returnvalue_2)))
            (if (> _returnvalue (`/Game/Excavator/BP_SaveGame.OpenLevelIndex` (`self.LastGameSave`)))
              (set `/Game/Excavator/BP_SaveGame.OpenLevelIndex` _returnvalue (`self.LastGameSave`))
              (set `self.Open Level Index` _returnvalue)
              (`self.SaveGame`))))
        (else
          ;[1 1 1] Уровень, который открывается, в случае если нет следующего уровня.
          (`GameplayStatics.OpenLevel` "Lvl_07_AdvencedQuadrantWalls__EndDemo"))))))

(fn `SaveGame`
  (`GameplayStatics.SaveGameToSlot` (`self.LastGameSave`) (`self.StaticSaveName`)))

(fn `UserConstructionScript`)