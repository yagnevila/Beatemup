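; BP_BallCollision is a physics-driven collision proxy that follows the ball collision socket on the player's BP_Excavator_2.
; Each Tick pulls component F toward that socket with a strong impulse scaled by offset and delta time, rather than attaching or teleporting it.
; F's hit and overlap events share a check for BP_StPanel_3 that only prints a debug message.
; An unused node for teleporting Soket remains disconnected.
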(event `self.ReceiveTick`
  (params (DeltaSeconds :type "Float (single-precision)"))
  (`PrimitiveComponent.AddImpulse` (`self.f`) (* (- (`SceneComponent.K2_GetComponentLocation` (`/Game/Excavator/BP_Excavator_2.BallColisionSoket` (cast `/Game/Excavator/BP_Excavator_2` (`GameplayStatics.GetPlayerCharacter` 0) :!pure true))) (`SceneComponent.K2_GetComponentLocation` (`self.f`))) (`GameplayStatics.GetWorldDeltaSeconds`) 6500000.0) "None" false))

(event `self.f.OnComponentHit`
  (params (HitComponent :type "PrimitiveComponent Object Reference") (OtherActor :type "Actor Object Reference") (OtherComp :type "PrimitiveComponent Object Reference") (NormalImpulse :type "Vector Structure") (Hit :type "HitResult Structure (by ref)"))
  (cast `/Game/Vampire-Panels/BP_StPanel_3` (stale `self.f.OnComponentBeginOverlap` OtherActor) :!label _label)
  (`KismetSystemLibrary.PrintString` "Hello"))

(event `self.f.OnComponentBeginOverlap`
  (params (OverlappedComponent :type "PrimitiveComponent Object Reference") (OtherActor :type "Actor Object Reference") (OtherComp :type "PrimitiveComponent Object Reference") (OtherBodyIndex :type Integer) (bFromSweep :type Boolean) (SweepResult :type "HitResult Structure (by ref)"))
  (goto _label))

(fn `UserConstructionScript`)