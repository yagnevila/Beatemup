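; Short-lived hitbox actor for a wide kick that hits enemies inside its Box.
; One tick after BeginPlay, it gathers overlapping actors and calls ToStan on each BP_Enemy with a vector along the Arrow, scaled by SpeedOfToss.
; It destroys itself after a brief delay.
; Tick and end-overlap are empty; unconnected nodes hold an unused approach for pushing enemies out of the box with LaunchCharacter.
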(event `self.ReceiveBeginPlay`
  (bind _overlappingactors (`PrimitiveComponent.GetOverlappingActors` (`self.Box`) null))
  (`|ExecutionSequence`
    (:`then_0`
      (`KismetSystemLibrary.DelayUntilNextTick`)
      (set `self.Overlapping Enemys` _overlappingactors)
      (for _array_element _overlappingactors
        (bind _asbp_enemy (cast `/Game/BP_Enemy` _array_element))
        (`/Game/BP_Enemy.To Stan` _asbp_enemy (`KismetMathLibrary.GreaterGreater_VectorRotator` (`KismetMathLibrary.MakeVector` (* (`self.SpeedOfToss`) 5.0)) (`SceneComponent.K2_GetComponentRotation` (`self.Arrow`))))))
    (:`then_1`
      (`KismetSystemLibrary.Delay` 2.0)
      (`self.K2_DestroyActor`))))

(event `self.ReceiveTick`
  (params (DeltaSeconds :type "Float (single-precision)"))
  ;[1 1 1] Код, аналогичный толканию как в длинном ударе. В плане не на определённое растояние всех — а только за пределы коллизии.
)

(event `self.Box.OnComponentEndOverlap`
  (params (OverlappedComponent :type "PrimitiveComponent Object Reference") (OtherActor :type "Actor Object Reference") (OtherComp :type "PrimitiveComponent Object Reference") (OtherBodyIndex :type Integer))
  ;[1 1 1] Код, аналогичный толканию как в длинном ударе. В плане не на определённое растояние всех — а только за пределы коллизии.
  ;;[1 1 1] Из той же оперы — код остановки при выходе из коллизии удара.
)

(fn `UserConstructionScript`)