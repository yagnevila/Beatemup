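; BP_Enemy is a melee enemy that chases the player in grid-like crowds, damaging and launching the player on overlap.
; Tick picks axis-biased AI move targets, while box hits snap aligned neighbours into lines.
; Visible neighbours set group membership and GroupVector, which recolours and slows front-rank enemies.
; ToStan, ignored in large groups, launches and briefly stuns the enemy, during which it pushes off neighbours perpendicular to the punch.
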(event `To Stan`
  (params (Vector :type "Vector Structure"))
  (bind _mesh (`self.Mesh`))
  (bind _box (`self.Box`))
  (bind _capsulecomponent (`self.CapsuleComponent`))
  ;[1 1 1 1 22] Эвент, которые переводит врага в состояние стана.
  ;
  ; Верхняя часть секверенса толкает врага в сторону,
  ; которую принимает эвент, то есть направление
  ; коллизии, которую создаёт игрок при ударе.
  ;
  ; (Тут хорошо бы сделать код для широко удара,
  ; по логике похожий на стабилизацию линии в ударе длинным.
  ; — на основе GroupVector, понимать находиться ли враг в линии
  ; относительно вектора широкого удара, и если нет, то толкать его сильнее)
  (if (not (`self.IsInGroup`))
    (`|ExecutionSequence`
      (:`then_0`
        (set `self.LastPunchVector` Vector)
        (`Timeline|Timeline` :!via `PlayFromStart`
          (:`Update`
            (`self.LaunchCharacter` (`KismetMathLibrary.GreaterGreater_VectorRotator` (* (`GameplayStatics.GetWorldDeltaSeconds`) Vector 10.0) (`KismetMathLibrary.MakeRotator` 0.0 0.0 (`KismetMathLibrary.RandomFloatInRange` -10.0 10.0)))))))
      (:`then_1`
        (set `self.IsInStan` true)
        (`PrimitiveComponent.SetMaterial` _mesh 0 "/DatasmithContent/Materials/AliasReference.AliasReference")
        (`PrimitiveComponent.SetCollisionEnabled` _box "NoCollision")
        (`CapsuleComponent.SetCapsuleRadius` _capsulecomponent 30.0 true))
      (:`then_2`
        (`KismetSystemLibrary.Delay` 2.7)
        (set `self.IsInStan` false)
        (`PrimitiveComponent.SetMaterial` _mesh 0 "/Game/Characters/Mannequins/Materials/Instances/Quinn/MI_Quinn_01.MI_Quinn_01")
        (`PrimitiveComponent.SetCollisionEnabled` _box "QueryAndPhysics")
        (`CapsuleComponent.SetCapsuleRadius` _capsulecomponent 40.0 true)))))

(event `self.Pain.OnComponentBeginOverlap`
  (params (OverlappedComponent :type "PrimitiveComponent Object Reference") (OtherActor :type "Actor Object Reference") (OtherComp :type "PrimitiveComponent Object Reference") (OtherBodyIndex :type Integer) (bFromSweep :type Boolean) (SweepResult :type "HitResult Structure (by ref)"))
  ;[1 1 1] Урон по главному героою
  (bind _asbp_third_person_character (cast `/Game/BP_ThirdPersonCharacter` OtherActor))
  (set `self.IsInAttack` true)
  (`GameplayStatics.ApplyDamage` _asbp_third_person_character 1.0)
  (`self.LaunchCharacter` _asbp_third_person_character (+ (`self.K2_GetActorLocation`) (* (`KismetMathLibrary.GreaterGreater_VectorRotator` (1.0 0.0 0.0) (`SceneComponent.K2_GetComponentRotation` (`self.Pain`))) 1500.0)) false false)
  (set `self.IsInAttack` false)
  (`KismetSystemLibrary.Delay` 0.5))

(event `self.ReceiveTick`
  (params (DeltaSeconds :type "Float (single-precision)"))
  (bind _returnvalue_location (`KismetMathLibrary.BreakTransform` (`self.GetTransform`)))
  (bind (_returnvalue_x _returnvalue_y) (`KismetMathLibrary.BreakVector` (`self.K2_GetActorLocation`)))
  (bind _returnvalue (`self.K2_GetActorLocation`))
  (bind (_lastpunchvector_x _lastpunchvector_y) (`KismetMathLibrary.BreakVector` (`self.LastPunchVector`)))
  (bind _charactermovement (`self.CharacterMovement`))
  (bind _mesh (`self.Mesh`))
  (bind _returnvalue_2 (`self.GetTransform` (`GameplayStatics.GetPlayerPawn` 0)))
  (bind _overlappingactors (`PrimitiveComponent.GetOverlappingActors` (`self.Capsule`) "BP_Enemy_C"))
  (bind (_returnvalue_x_2 _returnvalue_y_2) (`KismetMathLibrary.BreakVector` (`SceneComponent.GetForwardVector` (`self.CapsuleComponent`))))
  (bind _returnvalue_location_2 (`KismetMathLibrary.BreakTransform` (`self.GetTransform` (`GameplayStatics.GetPlayerPawn` 0))))
  (bind _returnvalue_3 (> (`KismetMathLibrary.Sqrt` (`KismetMathLibrary.Square` (- (.x (.location _returnvalue_2)) _returnvalue_x))) (`KismetMathLibrary.Sqrt` (`KismetMathLibrary.Square` (- (.y (.location _returnvalue_2)) _returnvalue_y)))))
  (`|ExecutionSequence`
    (:`then_0`
      ;[1 1 1] Код, которые задаёт искуственому интелекту врагу куда ходить.
      ;
      ; Так сложно, чтобы враги не застревали в друг-друге при передвижении в линии на игрока.
      (if (`self.IsInStan`)
        ;;[1 1 1] Код, которые останавливает AI движение врага.
        (`|AIMoveTo` self _returnvalue_location null)
        (else
          (`KismetSystemLibrary.Delay` 0.2)
          (`|AIMoveTo` self (`KismetMathLibrary.SelectVector` (`KismetMathLibrary.MakeVector` (`KismetMathLibrary.SelectFloat` (.x (.location _returnvalue_2)) _returnvalue_x _returnvalue_3) (`KismetMathLibrary.SelectFloat` _returnvalue_y (.y (.location _returnvalue_2)) _returnvalue_3) (.z (.location _returnvalue_2))) _returnvalue_location_2 (`self.IsActorsFrontToEachOther` (`GameplayStatics.GetPlayerCharacter` 0) self)) null))))
    (:`then_1`
      ;[1 1 1 1 22] Комплект нод отвечающий за подщёт врагов вокруг.
      ; Во-первых, для того, чтобы определять находиться ли актор в группе врагов.
      ; Во-вторых, в какой части группы он находиться — Group Vector
      (`KismetSystemLibrary.Delay` 0.2)
      (`|ExecutionSequence`
        (:`then_0`
          (set `self.GroupVector` (0.0 0.0))
          (set `self.EnemyAround` (`|MakeArray` null :!type "/Game/BP_Enemy Object Reference"))
          (for _array_element (`PrimitiveComponent.GetOverlappingActors` (`self.GroupEnemyCollision`) "BP_Enemy_C")
            (bind _returnvalue_4 (`self.K2_GetActorLocation` _array_element))
            (bind (_outhit _returnvalue_5) (`KismetSystemLibrary.LineTraceSingle` :`Start` _returnvalue_4 :`End` _returnvalue :`TraceChannel` "TraceTypeQuery1" :`DrawDebugType` "ForOneFrame"))
            (if (not _returnvalue_5)
              (`KismetArrayLibrary.Array_Add` (`self.EnemyAround`) (cast `/Game/BP_Enemy` _array_element :!pure true))
              (set `self.GroupVector` (+ (`KismetMathLibrary.Normal2D` (`KismetMathLibrary.MakeVector2D` (- (.x _returnvalue_4) (.x _returnvalue)) (- (.y _returnvalue_4) (.y _returnvalue)))) (`self.GroupVector`)))))
          (set `self.IsInGroup` (> (`KismetArrayLibrary.Array_Length` (`self.EnemyAround`)) 9)))
        (:`then_1`
          ;;[1 1 1] На основе GroupVector менает материал у врагов в передней части группы.
          ;; А также слегка уменьшает скорость этих авангардных врагов, для того чтобы группа меньше разбредалась.
          (if (> (`KismetMathLibrary.DotProduct2D` (`self.GroupVector`) (`KismetMathLibrary.MakeVector2D` _returnvalue_x_2 _returnvalue_y_2)) -0.5)
            (`PrimitiveComponent.SetMaterial` _mesh 1 "/Game/LevelPrototyping/Materials/MI_Solid_Blue.MI_Solid_Blue")
            (set `CharacterMovementComponent.MaxWalkSpeed` 200.0 _charactermovement)
            (else
              (`PrimitiveComponent.SetMaterial` _mesh 1 "/DatasmithContent/Materials/Arealight.Arealight")
              (set `CharacterMovementComponent.MaxWalkSpeed` 170.0 _charactermovement))))))
    (:`then_2`
      ;[1 1 1] Код, который проверяет застрял ли этот враг. Просто если не двигается.
      (`KismetSystemLibrary.Delay` 3.0)
      (`|ExecutionSequence`
        (:`then_0`
          (`KismetSystemLibrary.Delay` 1.0)
          (set `self.IsStopped` (== (stale _output_get) (`self.K2_GetActorLocation`))))
        (:`then_1`
          (bind _output_get (set `self.LocalLocation` (`self.K2_GetActorLocation`))))))
    (:`then_4`
      ;[1 1 1] Код, который пока этот враг в стане, каждыйе 0.03 секунды отталкивается от соседних врагов.
      ;
      ; Нужен для того, чтобы при толчке группы врагов в стену, они лучше распределялись в линию вдоль стены.
      (if (`self.IsInStan`)
        (`KismetSystemLibrary.Delay` 0.03)
        (if (> (`KismetArrayLibrary.Array_Length` _overlappingactors) 1)
          (for _array_element_2 _overlappingactors
            (bind (_returnvalue_x_3 _returnvalue_y_3) (`KismetMathLibrary.BreakVector` (* (`KismetMathLibrary.Normal` (- (`self.K2_GetActorLocation` _array_element_2) (`self.K2_GetActorLocation`))) -200.0)))
            (`self.LaunchCharacter` (`KismetMathLibrary.SelectVector` (`KismetMathLibrary.MakeVector` _returnvalue_x_3) (`KismetMathLibrary.MakeVector` 0.0 _returnvalue_y_3) (< (`KismetMathLibrary.Sqrt` (`KismetMathLibrary.Square` _lastpunchvector_x)) (`KismetMathLibrary.Sqrt` (`KismetMathLibrary.Square` _lastpunchvector_y)))))))))))

(event `self.Box.OnComponentHit`
  (params (HitComponent :type "PrimitiveComponent Object Reference") (OtherActor :type "Actor Object Reference") (OtherComp :type "PrimitiveComponent Object Reference") (NormalImpulse :type "Vector Structure") (Hit :type "HitResult Structure (by ref)"))
  (bind (_returnvalue_x _returnvalue_y) (`KismetMathLibrary.BreakVector` (`self.K2_GetActorLocation` OtherActor)))
  (bind (_returnvalue_x_2 _returnvalue_y_2) (`KismetMathLibrary.BreakVector` (`self.K2_GetActorLocation` self)))
  (bind _returnvalue (- _returnvalue_x _returnvalue_x_2))
  (bind _returnvalue_2 (- _returnvalue_y _returnvalue_y_2))
  ;[1 1 1] Этот код при соприкосновении с другим врагом, телепортирует
  ; одного из них на место, пенпендикулярное второму врагу.
  ;
  ; Это создаёт структуру врагов — то, что они ходят фигурами по сеточке.
  (cast `/Game/BP_Enemy` OtherActor)
  (if (and (not (or (`self.IsInStan`) (`self.IsStopped`))) (`self.IsActorsFrontToEachOther` OtherActor self 2.0))
    (`self.K2_SetActorLocation` OtherActor (+ (`self.K2_GetActorLocation` OtherActor) (* (`KismetMathLibrary.SelectVector` (`KismetMathLibrary.MakeVector` 0.0 _returnvalue_2) (`KismetMathLibrary.MakeVector` _returnvalue) (> (`KismetMathLibrary.Sqrt` (`KismetMathLibrary.Square` _returnvalue)) (`KismetMathLibrary.Sqrt` (`KismetMathLibrary.Square` _returnvalue_2)))) -1.0)) false false)))

(fn `UserConstructionScript`)